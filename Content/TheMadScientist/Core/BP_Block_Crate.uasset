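; BP_Block_Crate is a destructible crate block that loses one health point each time a projectile hits it.
; Its TakeDamage event decrements HealthPoints, then spawns a Niagara explosion at the crate and destroys it once health reaches zero.
; While health is at or below CrackThreshold but above zero, a DoOnce swaps in the cracked crate texture a single time through UpdateTexture.
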(event EventBeginPlay
  (|CallParentFunction) ; Ce nœud est désactivé et ne sera pas appelé.\nFaites glisser les broches pour générer des fonctionnalités.
)

(event Collision|EventActorBeginOverlap
  (params (OtherActor :type Actor%20Object%20Reference))
  (|CallParentFunction OtherActor) ; Ce nœud est désactivé et ne sera pas appelé.\nFaites glisser les broches pour générer des fonctionnalités.
)

(event EventTick
  (params (DeltaSeconds :type Float%20%28single-precision%29))
  (|CallParentFunction DeltaSeconds) ; Ce nœud est désactivé et ne sera pas appelé.\nFaites glisser les broches pour générer des fonctionnalités.
)

(event EventTakeDamage
  ;[0 0 0 0.5] Gère la prise de dégats lorsqu'on est touchés par un projectile
  (bind _result (Math|Integer|DecrementInt (Variables|Default|GetHealthPoints)) ; Retire un PV à chaque fois qu'un projectile touche la caisse
    (:%20%20
      (if (<= _result 0)
        (Niagara|SpawnSystematLocation "/Game/TheMadScientist/Core/NS_Explosion.NS_Explosion" (Transformation|GetActorLocation))
        (Actor|DestroyActor)
        (elif (<= _result (Variables|Default|GetCrackThreshold))
          (Utilities|FlowControl|DoOnce false
            (:Completed
              (CallFunction|UpdateTexture "/Game/TheMadScientist/Art/Interactables/Crate/T_Crate_Cracked.T_Crate_Cracked"))))))))

(fn ConstructionScript
  (|CallParentFunction))